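; Fishman character in Hungry Cat that recovers its displaced Fish and catches the cat carrying it.
; On capsule hit, a Fish away from its start spot is attached to the right hand socket with physics off.
; Hitting a cat holding it plays a fade, resets cat and fish positions, and registers the Basket as a sight stimulus.
; AI perception uses the head socket's location and rotation as its viewpoint.
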(event OnComponentHit(CapsuleComponent)
  (params (HitComponent :type Primitive%20Component%20Object%20Reference) (OtherActor :type Actor%20Object%20Reference) (OtherComp :type Primitive%20Component%20Object%20Reference) (NormalImpulse :type Vector :default "0, 0, 0") (Hit :type Hit%20Result%20Structure%20%28by%20ref%29))
  (bind _fish (Variables|Default|GetFish))
  (if (not (Math|Vector|Equal(Vector) (Variables|Default|GetFishDefaultPos) (Transformation|GetActorLocation (Variables|Default|GetFish)) 3e+01))
    (bind _asfish (Utilities|Casting|CastToFish OtherActor)
      (:then
        (if (Utilities|Enum|Equal(Enum) (Utilities|GetDisplayName OtherActor) "Fish")
          (Transformation|DetachFromActor _asfish "KeepWorld" "KeepWorld" "KeepWorld")
          (Transformation|AttachComponentToComponent _fish (Variables|Default|GetHand) "RightHandSocket" "SnapToTarget" "KeepWorld" "KeepWorld" true)
          (bind _asfish_2 (Utilities|Casting|CastToFish _fish))
          (Physics|SetSimulatePhysics (Variables|/Game/Hungry_Cat/Cat/PickableProps_BP.PickableProps_BP_C|GetProp _asfish_2) false)
          (Collision|SetCollisionProfileName (Variables|/Game/Hungry_Cat/Cat/PickableProps_BP.PickableProps_BP_C|GetProp _asfish_2) "OverlapOnlyPawn" :!class /Script/Engine.PrimitiveComponent)
          (Variables|Default|SetGotFish true)))
      (:CastFailed
        (if (Variables|Default|GetCat%20Not%20Catch)
          (bind _ascat_bp (Utilities|Casting|CastToCat_BP OtherActor))
          (if (and (Utilities|Enum|Equal(Enum) (Utilities|GetDisplayName (Variables|/Game/Hungry_Cat/Cat/Cat_BP.Cat_BP_C|GetPickedUpProp _ascat_bp)) "Fish") (Variables|/Game/Hungry_Cat/Cat/Cat_BP.Cat_BP_C|GetisHolding _ascat_bp))
            (Variables|Default|SetCat%20Not%20Catch false)
            (Input|DisableInput _ascat_bp (Game|GetPlayerController 0))
            (Default|ReleaseProp&SetPhysic _ascat_bp)
            (bind _returnvalue (Sequencer|Player|CreateLevelSequencePlayer "/Game/Hungry_Cat/Fishman/FadeInOut.FadeInOut"))
            (Sequencer|Player|Play _returnvalue :!class /Script/MovieScene.MovieSceneSequencePlayer)
            (Utilities|FlowControl|Delay 0.5)
            (Transformation|SetActorLocationAndRotation _ascat_bp (Variables|Default|GetCatDefaultPos) (Variables|Default|GetCatDefaultRot))
            (Variables|Default|SetCat%20Not%20Catch true)
            (Input|EnableInput _ascat_bp (Game|GetPlayerController 0))
            (CallFunction|SetFishonDefaultPos)
            (Class|AIPerceptionSystem|RegisterPerceptionStimuliSource "/Script/AIModule.AISense_Sight" (Variables|Default|GetBasket))))))))

(event EventBeginPlay
  (bind _fish (Variables|Default|GetFish))
  (Variables|Default|SetFishDefaultPos (Transformation|GetActorLocation _fish))
  (Variables|Default|SetFishDefaultRotation (Transformation|GetActorRotation _fish)))

(fn ConstructionScript)

(fn GetPerceptionLocRot
  (bind _mesh (Variables|Character|GetMesh))
  (bind _returnvalue (Transformation|GetSocketTransform _mesh "headSocket" "RTS_World"))
  (return (.location _returnvalue) (.rotation _returnvalue)))

(fn SetFishonDefaultPos
  (bind _fish (Variables|Default|GetFish))
  (bind _asfish (Utilities|Casting|CastToFish _fish))
  (Transformation|DetachFromActor _fish "KeepWorld" "KeepWorld" "KeepWorld")
  (Physics|SetSimulatePhysics (Variables|/Game/Hungry_Cat/Cat/PickableProps_BP.PickableProps_BP_C|GetProp _asfish) true)
  (Collision|SetCollisionProfileName (Variables|/Game/Hungry_Cat/Cat/PickableProps_BP.PickableProps_BP_C|GetProp _asfish) "PhysicsActor" :!class /Script/Engine.PrimitiveComponent)
  (Transformation|SetActorLocationAndRotation _fish (Variables|Default|GetFishDefaultPos) (Variables|Default|GetFishDefaultRotation)))