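; Fishman character for Hungry Cat that catches the fish in its hand and can return it to where it started.
; When its capsule hits the actor named "Fish", it attaches the fish to Hand, disables its physics and sets GotFish.
; SetFishOnDefaultPos detaches the fish, re-enables physics and restores the transform saved at BeginPlay.
; A check for the cat holding the fish exists but triggers nothing.
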(event OnComponentHit(CapsuleComponent)
  (params (HitComponent :type Primitive%20Component%20Object%20Reference) (OtherActor :type Actor%20Object%20Reference) (OtherComp :type Primitive%20Component%20Object%20Reference) (NormalImpulse :type Vector :default "0, 0, 0") (Hit :type Hit%20Result%20Structure%20%28by%20ref%29))
  (bind _fish (Variables|Default|GetFish))
  (Utilities|Casting|CastToFish OtherActor
    (:then
      (Development|PrintString (Utilities|GetDisplayName OtherActor))
      (if (Utilities|Enum|Equal(Enum) (Utilities|GetDisplayName OtherActor) "Fish")
        (Transformation|AttachComponentToComponent _fish (Variables|Default|GetHand) "None" "SnapToTarget" "KeepWorld" "KeepWorld" true)
        (bind _asfish (Utilities|Casting|CastToFish _fish))
        (Physics|SetSimulatePhysics (Variables|/Game/Hungry_Cat/Cat/PickableProps_BP.PickableProps_BP_C|GetProp _asfish) false)
        (Collision|SetCollisionProfileName (Variables|/Game/Hungry_Cat/Cat/PickableProps_BP.PickableProps_BP_C|GetProp _asfish) "OverlapOnlyPawn" :!class /Script/Engine.PrimitiveComponent)
        (Variables|Default|SetGotFish true)))
    (:CastFailed
      (bind _ascat_bp (Utilities|Casting|CastToCat_BP OtherActor))
      (if (and (Utilities|Enum|Equal(Enum) (Utilities|GetObjectName (Variables|/Game/Hungry_Cat/Cat/Cat_BP.Cat_BP_C|GetPickedUpProp _ascat_bp)) "Fish") (Variables|/Game/Hungry_Cat/Cat/Cat_BP.Cat_BP_C|GetisHolding _ascat_bp))
        _))))

(event EventBeginPlay
  (bind _fish (Variables|Default|GetFish))
  (Variables|Default|SetFishDefaultPos (Transformation|GetActorLocation _fish))
  (Variables|Default|SetFishDefaultRotation (Transformation|GetActorRotation _fish)))

(fn ConstructionScript)

(fn SetFishonDefaultPos
  (bind _fish (Variables|Default|GetFish))
  (bind _asfish (Utilities|Casting|CastToFish _fish))
  (Transformation|DetachFromActor _fish "KeepRelative" "KeepRelative" "KeepRelative")
  (Physics|SetSimulatePhysics (Variables|/Game/Hungry_Cat/Cat/PickableProps_BP.PickableProps_BP_C|GetProp _asfish) true)
  (Collision|SetCollisionProfileName (Variables|/Game/Hungry_Cat/Cat/PickableProps_BP.PickableProps_BP_C|GetProp _asfish) "PhysicsActor" :!class /Script/Engine.PrimitiveComponent)
  (Transformation|SetActorLocationAndRotation _fish (Variables|Default|GetFishDefaultPos) (Variables|Default|GetFishDefaultRotation)))