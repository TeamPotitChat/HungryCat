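; Camera actor for the Hungry Cat game, used as a child actor, that clamps the player camera's view pitch on BeginPlay.
; Tick only casts the parent to Cat_BP_Camera, with no further effect.
; Disconnected graphs hold unused experiments: sprint-triggered yaw recentering of the camera behind the parent through controller input, and an oscillating camera roll sway.
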(event EventBeginPlay
  (bind _returnvalue (Game|GetPlayerCameraManager 0))
  (Variables|Default|SetParentActor (Actor|GetParentActor))
  (Variables|/Script/Engine.PlayerCameraManager|SetViewPitchMax _returnvalue 1e+01)
  (Variables|/Script/Engine.PlayerCameraManager|SetViewPitchMin _returnvalue -4e+01))

(event EventTick
  (params (DeltaSeconds :type Float%20%28single-precision%29))
  (bind _ascat_bp_camera (Utilities|Casting|CastToCat_BP_Camera (Variables|Default|GetParentActor))))

(fn ConstructionScript)