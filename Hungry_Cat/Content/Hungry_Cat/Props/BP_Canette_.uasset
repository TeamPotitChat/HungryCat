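; BP_Canette_ is a can prop that gives impact feedback when the player's cat (Cat_BP) hits it.
; On a hit from the cat, it spawns a VFX system and a metallic sound at the hit location, then sets a Hit flag to block repeats.
; Tick clears that flag after a one-second Delay, acting as a simple cooldown between effects.
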(event EventBeginPlay)

(event Collision|EventActorBeginOverlap
  (params (OtherActor :type Actor%20Object%20Reference)))

(event EventTick
  (params (DeltaSeconds :type Float%20%28single-precision%29))
  (if (Variables|Default|GetHit)
    (Utilities|FlowControl|Delay 1.0)
    (Variables|Default|SetHit false)))

(event Collision|EventHit
  (params (MyComp :type Primitive%20Component%20Object%20Reference) (Other :type Actor%20Object%20Reference) (OtherComp :type Primitive%20Component%20Object%20Reference) (bSelfMoved :type Boolean) (HitLocation :type Vector :default "0, 0, 0") (HitNormal :type Vector :default "0, 0, 0") (NormalImpulse :type Vector :default "0, 0, 0") (Hit :type Hit%20Result%20Structure%20%28by%20ref%29))
  (Utilities|Casting|CastToCat_BP Other)
  (if (not (Variables|Default|GetHit))
    (Niagara|SpawnSystematLocation "/Game/Hungry_Cat/VFX_HIT_System.VFX_HIT_System" HitLocation)
    (Audio|SpawnSoundatLocation "/Game/Hungry_Cat/Audio/406562__anthousai__hit-metallic-01_Cue.406562__anthousai__hit-metallic-01_Cue" HitLocation "0, 0, 0" 1.0 1.0 0.0 0 0)
    (Variables|Default|SetHit true)))

(fn ConstructionScript)